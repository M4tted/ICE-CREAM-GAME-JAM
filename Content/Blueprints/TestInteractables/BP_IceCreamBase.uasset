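; BP_IceCreamBase is a base actor for an ice cream assembled from cone, cream, mix-in and topping components.
; Activating the cone, cream or mix-in component sets its active flag and adds a collision-free static mesh from that component's data struct.
; Toppings have no activation handler here.
; MakeIceCreamStruct records the display names of all four components in IceCreamStruct.
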(event OnComponentActivated(BPC_Cone)
  (params (Component :type Actor%20Component%20Object%20Reference) (bReset :type Boolean))
  (Variables|Default|SetConeActive true)
  (bind _returnvalue (AddComponent|AddStaticMeshComponent false))
  (Components|StaticMesh|SetStaticMesh _returnvalue (.StaticMesh (Utilities|Struct|BreakSTR_ConeInfo (Variables|/Game/Blueprints/TestInteractables/BPC_Cone.BPC_Cone_C|GetComponent%20Struct (Variables|Default|GetBPC_Cone)))))
  (Collision|SetCollisionEnabled _returnvalue "NoCollision"))

(event OnComponentActivated(BPC_IceCream)
  (params (Component :type Actor%20Component%20Object%20Reference) (bReset :type Boolean))
  (Variables|Default|SetCreamActive true)
  (bind _returnvalue (AddComponent|AddStaticMeshComponent false))
  (Components|StaticMesh|SetStaticMesh _returnvalue (.StaticMesh (Utilities|Struct|BreakSTR_ConeInfo (Variables|/Game/Blueprints/TestInteractables/BPC_IceCream.BPC_IceCream_C|GetIngredient%20Struct (Variables|Default|GetBPC_IceCream)))))
  (Collision|SetCollisionEnabled _returnvalue "NoCollision"))

(event OnComponentActivated(BPC_MixIns)
  (params (Component :type Actor%20Component%20Object%20Reference) (bReset :type Boolean))
  (Variables|Default|SetMixinsActive true)
  (bind _returnvalue (AddComponent|AddStaticMeshComponent false))
  (Components|StaticMesh|SetStaticMesh _returnvalue (.StaticMesh (Utilities|Struct|BreakSTR_ConeInfo (Variables|/Game/Blueprints/TestInteractables/BPC_MixIns.BPC_MixIns_C|GetIngredient%20Struct (Variables|Default|GetBPC_MixIns)))))
  (Collision|SetCollisionEnabled _returnvalue "NoCollision"))

(event Custom|Make%20Ice%20Cream%20Struct
  (Variables|Default|SetIce%20Cream%20Struct (Utilities|Struct|MakeSTR_OrderInfo (.DisplayName (Utilities|Struct|BreakSTR_ConeInfo (Variables|/Game/Blueprints/TestInteractables/BPC_Cone.BPC_Cone_C|GetComponent%20Struct (Variables|Default|GetBPC_Cone)))) (.DisplayName (Utilities|Struct|BreakSTR_ConeInfo (Variables|/Game/Blueprints/TestInteractables/BPC_IceCream.BPC_IceCream_C|GetIngredient%20Struct (Variables|Default|GetBPC_IceCream)))) (.DisplayName (Utilities|Struct|BreakSTR_ConeInfo (Variables|/Game/Blueprints/TestInteractables/BPC_MixIns.BPC_MixIns_C|GetIngredient%20Struct (Variables|Default|GetBPC_MixIns)))) (.DisplayName (Utilities|Struct|BreakSTR_ConeInfo (Variables|/Game/Blueprints/TestInteractables/BPC_Toppings.BPC_Toppings_C|GetIngredient%20Struct (Variables|Default|GetBPC_Toppings)))))))

(event EventBeginPlay)

(event Collision|EventActorBeginOverlap
  (params (OtherActor :type Actor%20Object%20Reference)))

(event EventTick
  (params (DeltaSeconds :type Float%20%28single-precision%29)))

(fn ConstructionScript)