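; BP_Cubes is an interactable mix-in ingredient that the player can pick up.
; On player interaction, it passes its IngredientStructData to the interacting actor through OnMixInPickup, then plays a 2D pickup sound.
; OnIngredientInteraction returns the same struct to callers.
; The construction script only calls its parent, and BeginPlay, overlap and Tick are disabled stubs.
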(event EventBeginPlay
  (|CallParentFunction) ; This node is disabled and will not be called.\nDrag off pins to build functionality.
)

(event Collision|EventActorBeginOverlap
  (params (OtherActor :type Actor%20Object%20Reference))
  (|CallParentFunction OtherActor) ; This node is disabled and will not be called.\nDrag off pins to build functionality.
)

(event EventTick
  (params (DeltaSeconds :type Float%20%28single-precision%29))
  (|CallParentFunction DeltaSeconds) ; This node is disabled and will not be called.\nDrag off pins to build functionality.
)

(event EventOnPlayerInteraction
  (params (Interacting%20Actor :type Player%20Character%20BP%20Object%20Reference))
  (Default|OnMixinPickup Interacting%20Actor (Variables|Default|GetIngredient%20Struct%20Data))
  (Audio|PlaySound2D "/Game/Audio/Item_PickUp.Item_PickUp" 1.0 1.0 0.0 0 0))

(fn ConstructionScript
  (|CallParentFunction))

(fn OnIngredientInteraction
  (return (Variables|Default|GetIngredient%20Struct%20Data)))