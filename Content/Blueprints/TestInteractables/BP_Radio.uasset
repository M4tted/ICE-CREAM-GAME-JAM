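; Interactable radio that starts playing audio on BeginPlay and lets the player toggle it off and on.
; A FlipFlop on player interaction alternates between stopping the audio and playing it from a saved resume time.
; Tick accumulates elapsed time while playing and copies it to the resume time while stopped, emulating pause and resume.
; Ingredient interaction is an empty stub.
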(event EventBeginPlay
  (Audio|Components|Audio|Play (Variables|Default|GetAudio) 0.0)
  (Variables|Default|SetTrackTimerOn true))

(event EventOnPlayerInteraction
  (params (Interacting%20Actor :type Player%20Character%20BP%20Object%20Reference))
  (bind _audio (Variables|Default|GetAudio))
  (Utilities|FlowControl|FlipFlop
    (:A
      (Audio|Components|Audio|Stop _audio)
      (Variables|Default|SetTrackTimerOn false))
    (:B
      (Audio|Components|Audio|Play _audio (Variables|Default|GetPlay%20Resume%20Time))
      (Variables|Default|SetTrackTimerOn true))))

(event EventTick
  (params (DeltaSeconds :type Float%20%28single-precision%29))
  (bind _output_get (Variables|Default|SetDelta%20Seconds DeltaSeconds))
  (if (Variables|Default|GetTrackTimerOn)
    (bind _output_get_2 (Variables|Default|Setelapsed%20time (+ _output_get (Variables|Default|Getelapsed%20time))))
    (else
      (Variables|Default|SetPlay%20Resume%20Time _output_get_2))))

(fn ConstructionScript)

(fn OnIngredientInteraction
  (return ""))