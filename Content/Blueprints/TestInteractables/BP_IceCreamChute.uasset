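; Ice cream delivery chute interactable that issues one order and times how fast the player fills it.
; After BeginPlay's delay it builds the order from the option arrays (RandomInteger(0) always picks the first entries) and starts a looping timer, which lets Tick spin the text.
; Interaction without ice cream shows the order widget.
; Matching cone, flavor and mix-ins, ignoring toppings, stops timing, submits the high score and destroys the ice cream.
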(event Custom|SpinText
  (bind _textrender (Variables|Default|GetTextRender))
  (if (Variables|Default|GetTimer%20Active)
    (if (== (.yaw (Variables|/Script/Engine.SceneComponent|GetRelativeRotation _textrender)) 3.6e+02)
      (Transformation|SetRelativeRotation _textrender "0, 0, 0" false false)
      (else
        (Transformation|AddRelativeRotation _textrender "0.000000,1.000000,0.000000" false false)))))

(event Custom|Get%20Order%20For%20Player
  (params (Player%20Ref :type Player%20Character%20BP%20Object%20Reference))
  (bind _returnvalue (UserInterface|CreateWidget "/Game/Blueprints/TestInteractables/WID_PendingOrder.WID_PendingOrder_C" 0 (Variables|Default|GetOrder%20Struct)))
  (bind _output_get (Variables|/Game/Blueprints/PlayerCharacter_BP.PlayerCharacter_BP_C|SetOrder%20Widget Player%20Ref _returnvalue))
  (UserInterface|Viewport|AddtoViewport _output_get 0))

(event Custom|Time%20Elapsed%20Counter
  (Variables|Default|SetTimeElapsed (+ (Variables|Default|GetTimeElapsed) 0.1))
  (Variables|Default|SetTimer%20Active true))

(event Custom|time%20elapsed%20timer
  (bind _returnvalue (Utilities|Time|SetTimerbyEvent (delegate Custom|Time%20Elapsed%20Counter) 0.1 true))
  (Variables|Default|SetElapsed%20Timer%20Handle _returnvalue))

(event Custom|Generate%20Order
  (Variables|Default|SetOrder%20Struct (Utilities|Struct|MakeSTR_OrderInfo (Utilities|Array|Get(acopy) (Variables|Default|GetCones) (Math|Random|RandomInteger 0)) (Utilities|Array|Get(acopy) (Variables|Default|GetFlavors) (Math|Random|RandomInteger 0)) (Utilities|Array|Get(acopy) (Variables|Default|GetMix%20Ins) (Math|Random|RandomInteger 0)) (Utilities|Array|Get(acopy) (Variables|Default|GetToppings) (Math|Random|RandomInteger 0))))
  (CallFunction|TimeElapsedTimer)
  (Variables|Default|SetpendingOrder true))

(event Custom|Pass%20Order)

(event EventTick
  (params (DeltaSeconds :type Float%20%28single-precision%29))
  (CallFunction|SpinText)
  (Development|PrintString (Utilities|String|ToString(Float) (Variables|Default|GetTimeElapsed)) true true "(R=0.000000,G=0.660000,B=1.000000,A=1.000000)" DeltaSeconds))

(event EventBeginPlay
  (Utilities|FlowControl|Delay 5.0)
  (CallFunction|GenerateOrder))

(event EventOnPlayerInteraction
  (params (Interacting%20Actor :type Player%20Character%20BP%20Object%20Reference))
  (bind _order_struct (Variables|Default|GetOrder%20Struct))
  (bind (_conetype _flavor _mixins) (Utilities|Struct|BreakSTR_OrderInfo _order_struct))
  (Utilities|IsValid (Variables|/Game/Blueprints/PlayerCharacter_BP.PlayerCharacter_BP_C|GetIce%20Cream%20Reference Interacting%20Actor)
    (:Is%20Valid
      (if (Math|Boolean|ANDBoolean (== (.ConeType (Utilities|Struct|BreakSTR_OrderInfo (Variables|/Game/Blueprints/TestInteractables/BP_IceCreamBase.BP_IceCreamBase_C|GetIce%20Cream%20Struct (Variables|/Game/Blueprints/PlayerCharacter_BP.PlayerCharacter_BP_C|GetIce%20Cream%20Reference Interacting%20Actor)))) _conetype) (== (.Flavor (Utilities|Struct|BreakSTR_OrderInfo (Variables|/Game/Blueprints/TestInteractables/BP_IceCreamBase.BP_IceCreamBase_C|GetIce%20Cream%20Struct (Variables|/Game/Blueprints/PlayerCharacter_BP.PlayerCharacter_BP_C|GetIce%20Cream%20Reference Interacting%20Actor)))) _flavor) (== (.MixIns (Utilities|Struct|BreakSTR_OrderInfo (Variables|/Game/Blueprints/TestInteractables/BP_IceCreamBase.BP_IceCreamBase_C|GetIce%20Cream%20Struct (Variables|/Game/Blueprints/PlayerCharacter_BP.PlayerCharacter_BP_C|GetIce%20Cream%20Reference Interacting%20Actor)))) _mixins))
        (Utilities|Time|InvalidateTimerHandle (Variables|Default|GetElapsed%20Timer%20Handle))
        (Default|SetHighScore (Variables|/Game/Blueprints/PlayerCharacter_BP.PlayerCharacter_BP_C|GetHigh%20Score%20Widget Interacting%20Actor) (Variables|Default|GetTimeElapsed))
        (Variables|Default|SetTimer%20Active false)
        (Variables|Default|SetTimeElapsed 0.0)
        (Actor|DestroyActor (Variables|/Game/Blueprints/PlayerCharacter_BP.PlayerCharacter_BP_C|GetIce%20Cream%20Reference Interacting%20Actor))
        (Variables|/Game/Blueprints/PlayerCharacter_BP.PlayerCharacter_BP_C|SetIce%20Cream%20Reference Interacting%20Actor 0)))
    (:Is%20Not%20Valid
      (if (Variables|Default|GetpendingOrder)
        (CallFunction|GetOrderforPlayer Interacting%20Actor)))))

(fn ConstructionScript)

(fn OnIngredientInteraction
  (return ""))