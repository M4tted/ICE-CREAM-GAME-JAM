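; BP_TestActor is a test interactable machine that randomly malfunctions until the player interacts with it to repair it.
; Each instance gathers the others at BeginPlay and starts a random malfunction timer.
; A malfunction fires every other machine's pause dispatcher, stopping their timers; repair fires their resume dispatchers and restarts all timers.
; Cube material colors show running, paused or malfunctioning state, and a text label shows the actor's name.
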(event Custom|SetMalfunctionTimer
  ;[1 1 1] Malfunction Timer
  (bind _returnvalue (Utilities|Time|SetTimerbyEvent (delegate Custom|MalfunctionHandler) (Math|Random|RandomFloatinRange 1.0 6.0)))
  (Variables|Default|SetMalfunctionTimerHandle _returnvalue))

(event Custom|MalfunctionHandler
  ;[1 1 1] Malfunction Timer
  (Variables|Default|SetMalfunctioning true)
  (Rendering|Material|SetMaterial (Variables|Default|GetCube) 0 "/Game/Materials/Basic/M_SolidColor_Red.M_SolidColor_Red")
  (for _array_element (Variables|Default|GetMachineActors)
    (Utilities|IsValid _array_element
      (:Is%20Valid
        (Default|CallPauseOperation _array_element)))))

(event Custom|get%20Other%20Machines
  ;[1 1 1] Get Other Machines Refs
  (bind _outactors (Actor|GetAllActorsOfClass "BP_TestActor_C"))
  (for (_array_element _array_index) _outactors
    (if (not (== _array_element self))
      (Utilities|Array|SetArrayElem (Variables|Default|GetMachineActors) _array_index _array_element true))))

(event Custom|Pause%20Operation
  ;[1 1 1] Pause Handlers
  (Utilities|Time|PauseTimerbyHandle (Variables|Default|GetMalfunctionTimerHandle))
  (Utilities|Time|InvalidateTimerHandle (Variables|Default|GetMalfunctionTimerHandle))
  (Rendering|Material|SetMaterial (Variables|Default|GetCube) 0 "/Game/Materials/Basic/M_SolidColor_Blue.M_SolidColor_Blue"))

(event Custom|Resume%20Operation
  ;[1 1 1] Pause Handlers
  (CallFunction|SetMalfunctionTimer)
  (Rendering|Material|SetMaterial (Variables|Default|GetCube) 0 "/Game/Materials/Basic/M_SolidColor_Green.M_SolidColor_Green"))

(event EventBeginPlay
  ;[1 1 1] Begin Play
  (CallFunction|GetOtherMachines)
  (CallFunction|SetMalfunctionTimer)
  (EventDispatchers|BindEventtoPauseOperation (EventDispatchers|CreateEvent :!event Custom|Pause%20Operation))
  (EventDispatchers|BindEventtoResumeOperation (EventDispatchers|CreateEvent :!event Custom|Resume%20Operation)))

(event EventOnPlayerInteraction
  (params (Interacting%20Actor :type Actor%20Object%20Reference))
  ;[1 1 1] On Player Interaction
  (if (Variables|Default|GetMalfunctioning)
    (Utilities|Time|InvalidateTimerHandle (Variables|Default|GetMalfunctionTimerHandle))
    (Variables|Default|SetMalfunctioning false)
    (Rendering|Material|SetMaterial (Variables|Default|GetCube) 0 "/Game/Materials/Basic/M_SolidColor_Green.M_SolidColor_Green")
    (CallFunction|SetMalfunctionTimer)
    (for _array_element (Variables|Default|GetMachineActors)
      (Utilities|IsValid _array_element
        (:Is%20Valid
          (Default|CallResumeOperation _array_element))))))

(fn ConstructionScript
  (Rendering|Components|TextRender|SetText (Variables|Default|GetTextRender) (Utilities|Text|ToText(String) (Utilities|GetDisplayName self))))

(fn OnIngredientInteraction
  (return ""))