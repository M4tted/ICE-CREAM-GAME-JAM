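; Interactable ice cream machine that combines a player's cone with cream they bring to it.
; A button press with the machine empty takes a cone-only item from the player and snaps it onto the holder.
; With a cone loaded and unpaused, a press restarts Niagara, waits the geometry cache's length, then copies cream-only ingredients onto the cone and destroys the carried item.
; An empty-handed press returns the filled, mixin-free cone to the player's socket.
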(event Custom|Do%20Machine%20Action
  (params (Player%20Ref :type Player%20Character%20BP%20Object%20Reference))
  (bind _icecreamref (Variables|Default|GetIceCreamRef))
  (bind _bpc_icecream (Variables|/Game/Blueprints/TestInteractables/BP_IceCreamBase.BP_IceCreamBase_C|GetBPC_IceCream _icecreamref))
  ;[1 1 1] Do Machine Action
  (bind _returnvalue (Animation|GetPlayLength (Variables|Default|GetGeometryCache)))
  (Niagara|ResetSystem (Variables|Default|GetNiagara))
  (Utilities|FlowControl|Delay _returnvalue)
  (if (Math|Boolean|ANDBoolean (== (Variables|/Game/Blueprints/TestInteractables/BP_IceCreamBase.BP_IceCreamBase_C|GetCreamActive (Variables|/Game/Blueprints/PlayerCharacter_BP.PlayerCharacter_BP_C|GetIce%20Cream%20Reference Player%20Ref)) true) (== (Variables|/Game/Blueprints/TestInteractables/BP_IceCreamBase.BP_IceCreamBase_C|GetConeActive (Variables|/Game/Blueprints/PlayerCharacter_BP.PlayerCharacter_BP_C|GetIce%20Cream%20Reference Player%20Ref)) false) (== (Variables|/Game/Blueprints/TestInteractables/BP_IceCreamBase.BP_IceCreamBase_C|GetMixinsActive (Variables|/Game/Blueprints/PlayerCharacter_BP.PlayerCharacter_BP_C|GetIce%20Cream%20Reference Player%20Ref)) false))
    (Variables|/Game/Blueprints/TestInteractables/BPC_IceCream.BPC_IceCream_C|SetIngredient%20Struct _bpc_icecream (Variables|/Game/Blueprints/TestInteractables/BPC_IceCream.BPC_IceCream_C|GetIngredient%20Struct (Variables|/Game/Blueprints/TestInteractables/BP_IceCreamBase.BP_IceCreamBase_C|GetBPC_IceCream (Variables|/Game/Blueprints/PlayerCharacter_BP.PlayerCharacter_BP_C|GetIce%20Cream%20Reference Player%20Ref))))
    (Utilities|IsValid (Variables|/Game/Blueprints/PlayerCharacter_BP.PlayerCharacter_BP_C|GetIce%20Cream%20Reference Player%20Ref)
      (:Is%20Valid
        (Components|Activation|SetActive _bpc_icecream true false)
        (Actor|DestroyActor (Variables|/Game/Blueprints/PlayerCharacter_BP.PlayerCharacter_BP_C|GetIce%20Cream%20Reference Player%20Ref))
        (Variables|/Game/Blueprints/PlayerCharacter_BP.PlayerCharacter_BP_C|SetIce%20Cream%20Reference Player%20Ref 0)
        (Variables|/Game/Blueprints/PlayerCharacter_BP.PlayerCharacter_BP_C|SetHandsFull Player%20Ref false)))))

(event Custom|Hand%20Back%20to%20Player
  (params (Player%20Ref :type Player%20Character%20BP%20Object%20Reference))
  ;[1 1 1] Hand Back to Player
  (if (Math|Boolean|ANDBoolean (== (Variables|/Game/Blueprints/TestInteractables/BP_IceCreamBase.BP_IceCreamBase_C|GetCreamActive (Variables|Default|GetIceCreamRef)) true) (== (Variables|/Game/Blueprints/TestInteractables/BP_IceCreamBase.BP_IceCreamBase_C|GetConeActive (Variables|Default|GetIceCreamRef)) true) (== (Variables|/Game/Blueprints/TestInteractables/BP_IceCreamBase.BP_IceCreamBase_C|GetMixinsActive (Variables|Default|GetIceCreamRef)) false))
    (bind _output_get (Variables|/Game/Blueprints/PlayerCharacter_BP.PlayerCharacter_BP_C|SetIce%20Cream%20Reference Player%20Ref (Variables|Default|GetIceCreamRef)))
    (Transformation|DetachFromActor _output_get "KeepRelative" "KeepRelative" "KeepRelative")
    (Transformation|AttachComponentToComponent (Variables|Default|GetIceCreamRef) (Variables|/Game/Blueprints/PlayerCharacter_BP.PlayerCharacter_BP_C|GetHolding%20Socket Player%20Ref) "None" "SnapToTarget" "SnapToTarget" "SnapToTarget" true)
    (Utilities|IsValid (Variables|Default|GetIceCreamRef)
      (:Is%20Valid
        (Variables|Default|SetIceCreamRef 0)))))

(event EventBeginPlay
  (|CallParentFunction) ; This node is disabled and will not be called.\nDrag off pins to build functionality.
)

(event Collision|EventActorBeginOverlap
  (params (OtherActor :type Actor%20Object%20Reference)))

(event EventTick
  (params (DeltaSeconds :type Float%20%28single-precision%29)))

(event EventButtonPress
  (params (Player%20Ref :type Player%20Character%20BP%20Object%20Reference))
  ;[1 1 1] Function Override - Button Press
  (Utilities|IsValid (Variables|Default|GetIceCreamRef)
    (:Is%20Valid
      (if (not (Variables|Default|GetisPaused))
        (Utilities|IsValid (Variables|/Game/Blueprints/PlayerCharacter_BP.PlayerCharacter_BP_C|GetIce%20Cream%20Reference Player%20Ref)
          (:Is%20Valid
            (CallFunction|DoMachineAction Player%20Ref))
          (:Is%20Not%20Valid
            (CallFunction|HandBacktoPlayer Player%20Ref)))))
    (:Is%20Not%20Valid
      (Utilities|IsValid (Variables|/Game/Blueprints/PlayerCharacter_BP.PlayerCharacter_BP_C|GetIce%20Cream%20Reference Player%20Ref)
        (:Is%20Valid
          (if (and (== (Variables|/Game/Blueprints/TestInteractables/BP_IceCreamBase.BP_IceCreamBase_C|GetConeActive (Variables|/Game/Blueprints/PlayerCharacter_BP.PlayerCharacter_BP_C|GetIce%20Cream%20Reference Player%20Ref)) true) (== (Variables|/Game/Blueprints/TestInteractables/BP_IceCreamBase.BP_IceCreamBase_C|GetCreamActive (Variables|/Game/Blueprints/PlayerCharacter_BP.PlayerCharacter_BP_C|GetIce%20Cream%20Reference Player%20Ref)) false))
            (bind _output_get (Variables|Default|SetIceCreamRef (Variables|/Game/Blueprints/PlayerCharacter_BP.PlayerCharacter_BP_C|GetIce%20Cream%20Reference Player%20Ref)))
            (Transformation|DetachFromActor _output_get "KeepRelative" "KeepRelative" "KeepRelative")
            (Transformation|AttachComponentToComponent _output_get (Variables|Default|GetIceCreamHolder) "None" "SnapToTarget" "SnapToTarget" "SnapToTarget" true)
            (Variables|/Game/Blueprints/PlayerCharacter_BP.PlayerCharacter_BP_C|SetIce%20Cream%20Reference Player%20Ref 0)
            (Variables|/Game/Blueprints/PlayerCharacter_BP.PlayerCharacter_BP_C|SetHandsFull Player%20Ref false)))))))

(fn ConstructionScript
  (|CallParentFunction))