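; Player character for an ice cream game that moves, looks, interacts and carries one item at a time.
; BeginPlay adds the Enhanced Input mapping context and score widget, and plays an entry sound.
; Interact fires a once-per-press camera line trace and sends an interaction message to the hit actor.
; Cone, cream and mix-in pickup events spawn an ice cream base on the holding socket if hands are empty, while throw-away destroys it.
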(event Custom|Movement
  ;[1 1 1] ADD INPUT CONTROLS
  (bind _asplayer_controller (Utilities|Casting|CastToPlayerController (Pawn|GetController)))
  (Utilities|IsValid (PlayerController|LocalPlayerSubsystems|GetEnhancedInputLocalPlayerSubsystem _asplayer_controller)
    (:Is%20Valid
      (Input|AddMappingContext (PlayerController|LocalPlayerSubsystems|GetEnhancedInputLocalPlayerSubsystem _asplayer_controller) "/Game/Inputs/IA_CharacterMovement.IA_CharacterMovement" 0 "(bIgnoreAllPressedKeysUntilRelease=True,bForceImmediately=False,bNotifyUserSettings=False)")
      (bind _returnvalue (UserInterface|CreateWidget "/Game/Blueprints/TestInteractables/WID_Score.WID_Score_C" (Game|GetPlayerController 0)))
      (Variables|Default|SetHigh%20Score%20Widget _returnvalue)
      (UserInterface|Viewport|AddtoViewport (Variables|Default|GetHigh%20Score%20Widget) 0))))

(event Input|EnhancedActionEvents|EnhancedInputActionIA_Move
  (params (ActionValue :type Vector%202D%20Structure) (ElapsedSeconds :type Float%20%28double-precision%29) (TriggeredSeconds :type Float%20%28double-precision%29) (InputAction :type Input%20Action%20Object%20Reference :default "/Game/Inputs/IA_Move.IA_Move"))
  ;[1 1 1] MOVEMENT
  (Pawn|Input|AddMovementInput (Transformation|GetActorRightVector) (.x ActionValue) false)
  (Pawn|Input|AddMovementInput (Transformation|GetActorForwardVector) (.y ActionValue) false))

(event Input|EnhancedActionEvents|EnhancedInputActionIA_Look
  (params (ActionValue :type Vector%202D%20Structure) (ElapsedSeconds :type Float%20%28double-precision%29) (TriggeredSeconds :type Float%20%28double-precision%29) (InputAction :type Input%20Action%20Object%20Reference :default "/Game/Inputs/IA_Look.IA_Look"))
  (Pawn|Input|AddControllerYawInput (.x ActionValue))
  (Pawn|Input|AddControllerPitchInput (.y ActionValue)))

(event Input|EnhancedActionEvents|EnhancedInputActionIA_Interact
  (params (ActionValue :type Boolean) (ElapsedSeconds :type Float%20%28double-precision%29) (TriggeredSeconds :type Float%20%28double-precision%29) (InputAction :type Input%20Action%20Object%20Reference :default "/Game/Inputs/IA_Interact.IA_Interact"))
  (bind _playcamera (Variables|Default|GetPlayCamera))
  (bind _returnvalue (Transformation|GetWorldLocation _playcamera))
  (:Started
    (Utilities|FlowControl|DoOnce false :!label _label
      (:Completed
        (bind _outhit (Collision|LineTraceByChannel _returnvalue (+ _returnvalue (* (Math|Vector|GetForwardVector _playcamera) 5e+02)) "TraceTypeQuery3" false 0 "None"))
        (bind _output_get (Variables|Default|SetHovered%20Actor (.HitActor (Collision|BreakHitResult _outhit))))
        (Class|BPIInteractions|OnPlayerInteraction(Message) _output_get self))))
  (:Canceled
    (goto _label Reset))
  (:Completed
    (goto _label Reset)))

(event EventTick
  (params (DeltaSeconds :type Float%20%28single-precision%29)))

(event EventOnConePickup
  (params (Cone%20Data :type STR%20Cone%20Info%20Structure))
  (if (not (Variables|Default|GetHandsFull))
    (bind _returnvalue (Game|SpawnActorfromClass "/Game/Blueprints/TestInteractables/BP_IceCreamBase.BP_IceCreamBase_C" (Transformation|GetRelativeTransform (Variables|Default|GetHolding%20Socket)) "Undefined" "MultiplyWithRoot" 0 0))
    (Variables|Default|SetHandsFull true)
    (bind _output_get (Variables|Default|SetIce%20Cream%20Reference _returnvalue))
    (Variables|/Game/Blueprints/TestInteractables/BPC_Cone.BPC_Cone_C|SetComponent%20Struct (Variables|/Game/Blueprints/TestInteractables/BP_IceCreamBase.BP_IceCreamBase_C|GetBPC_Cone _output_get) Cone%20Data)
    (Components|Activation|Activate (Variables|/Game/Blueprints/TestInteractables/BP_IceCreamBase.BP_IceCreamBase_C|GetBPC_Cone _output_get) false)
    (Transformation|AttachComponentToComponent _returnvalue (Variables|Default|GetHolding%20Socket) "None" "SnapToTarget" "SnapToTarget" "SnapToTarget" true)))

(event EventOnCreamPickup
  (params (Cream%20Info :type STR%20Cone%20Info%20Structure))
  (if (not (Variables|Default|GetHandsFull))
    (bind _returnvalue (Game|SpawnActorfromClass "/Game/Blueprints/TestInteractables/BP_IceCreamBase.BP_IceCreamBase_C" (Transformation|GetRelativeTransform (Variables|Default|GetHolding%20Socket)) "Undefined" "MultiplyWithRoot" 0 0))
    (Variables|Default|SetHandsFull true)
    (bind _output_get (Variables|Default|SetIce%20Cream%20Reference _returnvalue))
    (Variables|/Game/Blueprints/TestInteractables/BPC_IceCream.BPC_IceCream_C|SetIngredient%20Struct (Variables|/Game/Blueprints/TestInteractables/BP_IceCreamBase.BP_IceCreamBase_C|GetBPC_IceCream _output_get) Cream%20Info)
    (Components|Activation|Activate (Variables|/Game/Blueprints/TestInteractables/BP_IceCreamBase.BP_IceCreamBase_C|GetBPC_IceCream _output_get) false)
    (Transformation|AttachComponentToComponent _returnvalue (Variables|Default|GetHolding%20Socket) "None" "SnapToTarget" "SnapToTarget" "SnapToTarget" true)))

(event EventBeginPlay
  (CallFunction|Movement)
  (Audio|PlaySound2D "/Game/Audio/EnteringGame.EnteringGame" 1.0 1.0 0.0 0 0))

(event EventOnMixinPickup
  (params (Mix%20Info :type STR%20Cone%20Info%20Structure))
  (if (not (Variables|Default|GetHandsFull))
    (bind _returnvalue (Game|SpawnActorfromClass "/Game/Blueprints/TestInteractables/BP_IceCreamBase.BP_IceCreamBase_C" (Transformation|GetRelativeTransform (Variables|Default|GetHolding%20Socket)) "Undefined" "MultiplyWithRoot" 0 0))
    (Variables|Default|SetHandsFull true)
    (bind _output_get (Variables|Default|SetIce%20Cream%20Reference _returnvalue))
    (Variables|/Game/Blueprints/TestInteractables/BPC_MixIns.BPC_MixIns_C|SetIngredient%20Struct (Variables|/Game/Blueprints/TestInteractables/BP_IceCreamBase.BP_IceCreamBase_C|GetBPC_MixIns _output_get) Mix%20Info)
    (Components|Activation|Activate (Variables|/Game/Blueprints/TestInteractables/BP_IceCreamBase.BP_IceCreamBase_C|GetBPC_MixIns _output_get) false)
    (Transformation|AttachComponentToComponent _returnvalue (Variables|Default|GetHolding%20Socket) "None" "SnapToTarget" "SnapToTarget" "SnapToTarget" true)))

(event EventOnThrowAway
  (Actor|DestroyActor (Variables|Default|GetIce%20Cream%20Reference))
  (Variables|Default|SetIce%20Cream%20Reference 0)
  (Variables|Default|SetHandsFull false))

(fn ConstructionScript)

(fn OnIngredientInteraction
  (return ""))